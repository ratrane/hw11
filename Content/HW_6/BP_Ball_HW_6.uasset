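; Bouncing ball actor that moves along its Direction at Speed and slows as it hits surfaces.
; Tick moves it with a swept world offset, and a blocking hit reflects Direction about the surface normal.
; BeginPlay stores a tenth of Speed in a variable named "10" and replaces non-positive Speed with MinSpeed.
; Each bounce subtracts that step, or sets Speed to it once at or below MinSpeed.
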(event `self.ReceiveBeginPlay`
  (`self.SpeedCheck`))

(event `self.ReceiveTick`
  (params (DeltaSeconds :type "Float (single-precision)"))
  (bind _sweephitresult (`self.K2_AddActorWorldOffset` (* (* (`self.Direction`) (`self.Speed`)) DeltaSeconds) true))
  (bind (_bblockinghit _binitialoverlap _time _distance _location _impactpoint _normal) (`GameplayStatics.BreakHitResult` _sweephitresult))
  (if _bblockinghit
    (set `self.Direction` (`KismetMathLibrary.GetReflectionVector` (`self.Direction`) _normal))
    (`self.ChangingSpeed`)))

(fn `ChangingSpeed`
  (if (<= (`self.Speed`) (`self.MinSpeed`))
    (set `self.Speed` (`self.10%`))
    (else
      (set `self.Speed` (- (`self.Speed`) (`self.10%`))))))

(fn `SpeedCheck`
  (set `self.10%` (* (`self.Speed`) 0.1))
  (if (<= (`self.Speed`) 0.0)
    (set `self.Speed` (`self.MinSpeed`))))

(fn `UserConstructionScript`)