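; BP_Pawn is a player pawn that slides sideways along the Y axis and spawns a ball for play.
; The MoveRight axis sets only the direction, applying a fixed swept offset per input event, so speed is not scaled by delta time.
; BeginPlay calls SpawnBall, which spawns BP_Ball_HW8 at the capsule, stores it as PlayingBall and binds to its OnDead event.
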(event `InputAxis|MoveRight`
  (params (AxisValue :type "Float (single-precision)"))
  ;[1 1 1] Movement
  (if (< AxisValue 0.0)
    (`self.K2_AddActorWorldOffset` (0.0 -50.0 0.0) true)))

(event `InputAxis|MoveRight`
  (params (AxisValue :type "Float (single-precision)"))
  ;[1 1 1] Movement
  (if (> AxisValue 0.0)
    (`self.K2_AddActorWorldOffset` (0.0 50.0 0.0) true)))

(event `self.ReceiveBeginPlay`
  (`self.SpawnBall`))

(fn `SpawnBall`
  (bind _returnvalue_location (`KismetMathLibrary.BreakTransform` (`SceneComponent.K2_GetComponentToWorld` (`self.Capsule`))))
  (bind _returnvalue (`|SpawnActorFromClass` "/Game/HW_8/BP_Ball_HW8.BP_Ball_HW8_C" (`KismetMathLibrary.MakeTransform` _returnvalue_location) "AlwaysSpawn" "OverrideRootScale" null null))
  (bind _output_get (set `self.PlayingBall` _returnvalue))
  (add `/Game/HW_8/BP_Ball_HW8.OnDead` _output_get (`|CreateDelegate` :!event `SpawnBall`)))

(fn `UserConstructionScript`)