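; BP_Block is a breakable block that takes two hits from BP_Ball_HW8 to destroy.
; The first hit plays a high-pitched shutter sound, sets the boolean HitCount and swaps the cube's material to show damage.
; The second hit plays the sound at normal pitch, destroys the block and rolls a random number, spawning a BP_BonusBlock at its location roughly one time in three.
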(event `self.ReceiveHit`
  (params (MyComp :type "PrimitiveComponent Object Reference") (Other :type "Actor Object Reference") (OtherComp :type "PrimitiveComponent Object Reference") (bSelfMoved :type Boolean) (HitLocation :type "Vector Structure") (HitNormal :type "Vector Structure") (NormalImpulse :type "Vector Structure") (Hit :type "HitResult Structure (by ref)"))
  (cast `/Game/HW_9/BP_Ball_HW8` Other)
  (if (`self.HitCount`)
    (`GameplayStatics.PlaySound2D` "/Engine/VREditor/Sounds/UI/Camera_Shutter.Camera_Shutter" 1.0 1.0 0.0 null null)
    (`self.K2_DestroyActor`)
    (set `self.BonusChance` (`KismetMathLibrary.RandomIntegerInRange` 0 100))
    (if (>= (`self.BonusChance`) 66)
      (`|SpawnActorFromClass` "/Game/HW_9/BP_BonusBlock.BP_BonusBlock_C" (`KismetMathLibrary.Conv_VectorToTransform` (`self.K2_GetActorLocation`)) "AlwaysSpawn" "OverrideRootScale" null null)
      (else
        (set `self.BonusChance` 0)))
    (else
      (`GameplayStatics.PlaySound2D` "/Engine/VREditor/Sounds/UI/Camera_Shutter.Camera_Shutter" 1.0 3.0 0.0 null null)
      (set `self.HitCount` true)
      (`PrimitiveComponent.SetMaterial` (`self.Cube`) 0 "/Engine/VREditor/UI/ArrowMaterial.ArrowMaterial"))))

(fn `UserConstructionScript`)