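; BP_Blocks is a spawner actor that lays out a grid of BP_Block actors when play begins.
; BeginPlay runs nested loops over X and Y and spawns a block at the actor's location, offset on the X and Y axes by each index times Padding.
; Both loops include their end value, and the construction script is empty, so the grid only appears at runtime.
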(event `self.ReceiveBeginPlay`
  (for _index (range (+ (`self.X`) 1))
    (for _index_2 (range (+ (`self.Y`) 1))
      (`|SpawnActorFromClass` "/Game/HW_9/BP_Block.BP_Block_C" (`KismetMathLibrary.MakeTransform` (+ (`self.K2_GetActorLocation`) (`KismetMathLibrary.MakeVector` (`KismetMathLibrary.Conv_IntToDouble` (* _index (`self.Padding`))) (`KismetMathLibrary.Conv_IntToDouble` (* _index_2 (`self.Padding`)))))) "Undefined" "OverrideRootScale" null null))))

(fn `UserConstructionScript`)