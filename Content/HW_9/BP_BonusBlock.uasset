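; BP_BonusBlock is a moving bonus pickup that spawns an extra ball when it hits BP_Caretka.
; Tick moves it by a swept offset from Direction and Speed, scaled by delta time.
; A hit with BP_Caretka destroys it and spawns a BP_Ball_HW8 at its location, regardless of collisions.
; Overlapping a KillZVolume destroys it without spawning a ball.
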(event `self.ReceiveTick`
  (params (DeltaSeconds :type "Float (single-precision)"))
  (`self.K2_AddActorLocalOffset` (* (* (`self.Direction`) (`self.Speed`)) DeltaSeconds) true))

(event `self.ReceiveActorBeginOverlap`
  (params (OtherActor :type "Actor Object Reference"))
  (cast `KillZVolume` OtherActor)
  (`self.K2_DestroyActor`))

(event `self.ReceiveHit`
  (params (MyComp :type "PrimitiveComponent Object Reference") (Other :type "Actor Object Reference") (OtherComp :type "PrimitiveComponent Object Reference") (bSelfMoved :type Boolean) (HitLocation :type "Vector Structure") (HitNormal :type "Vector Structure") (NormalImpulse :type "Vector Structure") (Hit :type "HitResult Structure (by ref)"))
  (cast `/Game/HW_9/BP_Caretka` Other)
  (`self.K2_DestroyActor`)
  (`|SpawnActorFromClass` "/Game/HW_9/BP_Ball_HW8.BP_Ball_HW8_C" (`KismetMathLibrary.Conv_VectorToTransform` (`self.K2_GetActorLocation`)) "AlwaysSpawn" "OverrideRootScale" null null))

(fn `UserConstructionScript`)